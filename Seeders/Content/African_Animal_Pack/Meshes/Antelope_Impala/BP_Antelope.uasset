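; Antelope actor that runs along its spline and jumps twice shortly after play begins.
; A timeline, with play rate set by Time, moves the skeletal mesh along the spline, matching its rotation with inverted pitch and a yaw offset.
; Each jump spikes the BlendSpace value, which Tick counts down per frame, presumably to drive animation blending.
; Direct jump and run animation calls are left unconnected.
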(event `self.ReceiveBeginPlay`
  (`|ExecutionSequence`
    (:`then_0`
      (`self.AntelopeRun`))
    (:`then_1`
      (`KismetSystemLibrary.Delay` 2.0)
      (`self.Jump`)
      (`KismetSystemLibrary.Delay` 2.0)
      (`self.Jump`))))

(event `AntelopeRun`
  (`TimelineComponent.SetPlayRate` (`self.Timeline`) (`self.Time`))
  (bind (_direction _alpha) (`Timeline|Timeline`)
    (:`Update`
      (bind _returnvalue (`KismetMathLibrary.Lerp` 0.0 (`SplineComponent.GetSplineLength` (`self.Spline`)) _alpha))
      (bind (_returnvalue_roll _returnvalue_pitch _returnvalue_yaw) (`KismetMathLibrary.BreakRotator` (`KismetMathLibrary.ComposeRotators` (`SplineComponent.GetRotationAtDistanceAlongSpline` (`self.Spline`) _returnvalue "Local"))))
      (`SceneComponent.K2_SetRelativeTransform` (`self.SkeletalMesh`) (`KismetMathLibrary.MakeTransform` (`SplineComponent.GetLocationAtDistanceAlongSpline` (`self.Spline`) _returnvalue "Local") (`KismetMathLibrary.MakeRotator` _returnvalue_roll (* _returnvalue_pitch -1.0) (+ _returnvalue_yaw 625.0)) (`SceneComponent.RelativeScale3D` (`self.SkeletalMesh`))) false false))))

(event `self.ReceiveTick`
  (params (DeltaSeconds :type "Float (single-precision)"))
  (if (`self.Blendspacetrigger`)
    (set `self.BlendSpace` (- (`self.BlendSpace`) 1.0))
    (if (< (`self.BlendSpace`) 2.0)
      (set `self.Blendspacetrigger` false))))

(event `Jump`
  (set `self.BlendSpace` 100.0)
  (set `self.Blendspacetrigger` true))

(fn `UserConstructionScript`)