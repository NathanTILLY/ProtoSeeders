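; AI controller for the impala antelope NPC that runs its behavior tree.
; On BeginPlay it optionally waits for the pawn's configured duration, starts BTAntelope, then copies the pawn's random-or-controlled movement flag to the blackboard.
; A GoThroughCheckpoints event writes the next checkpoint's location from the pawn's list to DefinedLocation, stopping at the end without looping.
; Pawn settings are read through casts to TrueAntelopeNPC.
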(event `self.ReceiveBeginPlay`
  (bind _astrue_antelope_npc (cast `/Game/African_Animal_Pack/Meshes/Antelope_Impala/TrueAntelopeNPC` (`self.K2_GetPawn`) :!pure true))
  (`KismetSystemLibrary.Delay` 0.1)
  (if (`/Game/Blueprint/AI/NPC_AI/BP_ParentNPC.WaitTime` _astrue_antelope_npc)
    (`KismetSystemLibrary.Delay` (`/Game/Blueprint/AI/NPC_AI/BP_ParentNPC.WaitDuration` _astrue_antelope_npc)))
  ;[1 0.159 0] WhenCopyingChangeThat
  (`self.RunBehaviorTree` "/Game/African_Animal_Pack/Meshes/Antelope_Impala/BTAntelope.BTAntelope")
  ;[1 1 1] Handle wheter random or controlled
  (`KismetSystemLibrary.Delay` 0.2)
  (`BlackboardComponent.SetValueAsBool` (`AIBlueprintHelperLibrary.GetBlackboard` null) "RandomTrueOrControlledFalse" (`/Game/Blueprint/AI/NPC_AI/BP_ParentNPC.RandomTrueOrControlledFalse` (cast `/Game/African_Animal_Pack/Meshes/Antelope_Impala/TrueAntelopeNPC` (`self.K2_GetPawn`) :!pure true))))

(event `self.ReceiveTick`
  (params (DeltaSeconds :type "Float (single-precision)")))

(event `GoThroughCheckpoints`
  (bind _checkpoints (`/Game/Blueprint/AI/NPC_AI/BP_ParentNPC.Checkpoints` (cast `/Game/African_Animal_Pack/Meshes/Antelope_Impala/TrueAntelopeNPC` (`self.K2_GetPawn`) :!pure true)))
  (if (not (>= (`self.incrementationList`) (`KismetArrayLibrary.Array_Length` _checkpoints)))
    (`BlackboardComponent.SetValueAsVector` (`AIBlueprintHelperLibrary.GetBlackboard` null) "DefinedLocation" (`self.K2_GetActorLocation` (`|GetArrayItem` _checkpoints (`self.incrementationList`))))
    (`/Engine/EditorBlueprintResources/StandardMacros.IncrementInt` (`self.incrementationList`))))

(fn `UserConstructionScript`
  (`parent.UserConstructionScript`))