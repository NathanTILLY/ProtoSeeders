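; BP_Hyena is a hyena actor that moves its skeletal mesh along a spline, starting on BeginPlay.
; HyenaWalk plays a timeline at a rate set by the Time variable, mapping its alpha to distance along the spline.
; Each update sets the mesh's relative transform from the spline's local location and rotation, negating pitch and offsetting yaw to orient the mesh while keeping its scale.
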(event `self.ReceiveBeginPlay`
  (`self.HyenaWalk`))

(event `HyenaWalk`
  (`TimelineComponent.SetPlayRate` (`self.Timeline`) (`self.Time`))
  (bind (_direction _alpha) (`Timeline|Timeline`)
    (:`Update`
      (bind _returnvalue (`KismetMathLibrary.Lerp` 0.0 (`SplineComponent.GetSplineLength` (`self.Spline`)) _alpha))
      (bind (_returnvalue_roll _returnvalue_pitch _returnvalue_yaw) (`KismetMathLibrary.BreakRotator` (`KismetMathLibrary.ComposeRotators` (`SplineComponent.GetRotationAtDistanceAlongSpline` (`self.Spline`) _returnvalue "Local"))))
      (`SceneComponent.K2_SetRelativeTransform` (`self.SkeletalMesh`) (`KismetMathLibrary.MakeTransform` (`SplineComponent.GetLocationAtDistanceAlongSpline` (`self.Spline`) _returnvalue "Local") (`KismetMathLibrary.MakeRotator` _returnvalue_roll (* _returnvalue_pitch -1.0) (+ _returnvalue_yaw 625.0)) (`SceneComponent.RelativeScale3D` (`self.SkeletalMesh`))) false false))))

(fn `UserConstructionScript`)