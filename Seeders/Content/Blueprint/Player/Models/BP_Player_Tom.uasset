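; Player character Blueprint for Tom that adds a CPR action.
; While the CPR input action triggers, it sets the DoCPR flag and zeroes the walk speed to hold the character in place.
; When the action completes or is canceled, a shared fixed delay of several seconds runs before it clears the flag and restores walk speed.
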(event `EnhancedInput|/Game/Blueprint/Player/Input/Actions/CPR`
  (params (ActionValue :type Boolean) (ElapsedSeconds :type "Float (double-precision)") (TriggeredSeconds :type "Float (double-precision)") (InputAction :type "InputAction Object Reference" :default "/Game/Blueprint/Player/Input/Actions/CPR.CPR"))
  (:`Triggered`
    (set `self.DoCPR` true)
    (set `CharacterMovementComponent.MaxWalkSpeed` 0.0 (`self.CharacterMovement`)))
  (:`Canceled`
    (`KismetSystemLibrary.Delay` 8.63 :!label _label)
    (set `self.DoCPR` false)
    (set `CharacterMovementComponent.MaxWalkSpeed` 500.0 (`self.CharacterMovement`)))
  (:`Completed`
    (goto _label)))

(fn `UserConstructionScript`
  (`parent.UserConstructionScript`))