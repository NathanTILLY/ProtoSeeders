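; BP_Marshaller is an event actor whose Boule component bobs gently up and down as a floating animation.
; Tick calls the Floating event every frame, which chains two latent MoveComponentTo moves with eased timing, one upward and one downward.
; Each target is an offset from the component's current relative location, with no stored origin, and rotation is left unchanged.
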(event `self.ReceiveTick`
  (params (DeltaSeconds :type "Float (single-precision)"))
  (`self.Floating`))

(event `Floating`
  (bind _boule (`self.Boule`))
  (bind _boule_2 (`self.Boule`))
  (bind _returnvalue (`SceneComponent.GetRelativeTransform` _boule_2))
  (bind _returnvalue_2 (`SceneComponent.GetRelativeTransform` _boule))
  (`KismetSystemLibrary.MoveComponentTo` _boule_2 (`KismetMathLibrary.MakeVector` (.x (.location _returnvalue)) (.y (.location _returnvalue)) (+ (.z (.location _returnvalue)) 10.0)) (.rotation _returnvalue) true true 1.0)
  (`KismetSystemLibrary.MoveComponentTo` _boule (`KismetMathLibrary.MakeVector` (.x (.location _returnvalue_2)) (.y (.location _returnvalue_2)) (+ (.z (.location _returnvalue_2)) -10.0)) (.rotation _returnvalue_2) true true 1.0))

(fn `UserConstructionScript`)