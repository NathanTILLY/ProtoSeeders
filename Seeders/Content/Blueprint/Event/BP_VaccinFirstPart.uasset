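; BP_VaccinFirstPart is a timed scripted animation of the first part of a vaccination, starting on BeginPlay.
; Three delayed sequence branches run in parallel: a timeline moves Syringe1 to draw the vaccine, the skeletal mesh briefly plays at double speed, and the Pfizer vial detaches to fall into a bin with physics.
; The syringe offset accumulates along relative Y every timeline update, making its travel frame-rate dependent.
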(event `self.ReceiveBeginPlay`
  (bind _syringe1 (`self.Syringe1`))
  (bind _pfizer (`self.Pfizer`))
  (bind (_relativelocation_x _relativelocation_y _relativelocation_z) (`KismetMathLibrary.BreakVector` (`SceneComponent.RelativeLocation` _syringe1)))
  (`|ExecutionSequence`
    (:`then_0`
      ;[1 1 1] Drop the vial in the bin
      (`KismetSystemLibrary.Delay` 3.5)
      (`SceneComponent.K2_DetachFromComponent` (`self.Pfizer`) "KeepWorld" "KeepWorld" "KeepWorld" true)
      (`PrimitiveComponent.SetSimulatePhysics` _pfizer true)
      (`PrimitiveComponent.SetEnableGravity` _pfizer true))
    (:`then_1`
      ;[1 1 1] Take in the syringe the vaccin
      (`KismetSystemLibrary.Delay` 1.0)
      (bind (_direction _newtrack_0) (`Timeline|Timeline_1`)
        (:`Update`
          (`SceneComponent.K2_SetRelativeLocation` _syringe1 (`KismetMathLibrary.MakeVector` _relativelocation_x (+ _relativelocation_y (`KismetMathLibrary.Lerp` 0.0 1.0 _newtrack_0)) _relativelocation_z) false false))))
    (:`then_2`
      (`KismetSystemLibrary.Delay` 2.0)
      (`SkeletalMeshComponent.SetPlayRate` (`self.SkeletalMesh`) 2.0)
      (`KismetSystemLibrary.Delay` 0.5)
      (`SkeletalMeshComponent.SetPlayRate` (`self.SkeletalMesh`) 1.0))))

(fn `UserConstructionScript`)