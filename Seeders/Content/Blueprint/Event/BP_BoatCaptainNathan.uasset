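; Boat actor that drives a Zodiac along a spline path shortly after play begins.
; The Path timeline, rate set by Time, moves Core along the spline, yawing it with a 90-degree offset and turning negated path pitch into roll.
; Tick calls Floating to ease Boule up and down; its trailing random Delay leads to nothing.
; FloatingBoat defines the same bob for Zodiac but is not called here.
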(event `self.ReceiveBeginPlay`
  (`KismetSystemLibrary.Delay` 0.2)
  (`self.ZodiacGoVROUM`))

(event `ZodiacGoVROUM`
  (`TimelineComponent.SetPlayRate` (`self.Path`) (`self.Time`))
  (bind (_direction _alpha) (`Timeline|Path`)
    (:`Update`
      (bind _returnvalue (`KismetMathLibrary.Lerp` 0.0 (`SplineComponent.GetSplineLength` (`self.Spline`)) _alpha))
      (bind (_returnvalue_roll _returnvalue_pitch _returnvalue_yaw) (`KismetMathLibrary.BreakRotator` (`KismetMathLibrary.ComposeRotators` (`SplineComponent.GetRotationAtDistanceAlongSpline` (`self.Spline`) _returnvalue "Local") (struct :`Yaw` 90.0))))
      (`SceneComponent.K2_SetRelativeTransform` (`self.Core`) (`KismetMathLibrary.MakeTransform` (`SplineComponent.GetLocationAtDistanceAlongSpline` (`self.Spline`) _returnvalue "Local") (`KismetMathLibrary.MakeRotator` (* _returnvalue_pitch -1.0) 0.0 _returnvalue_yaw) (`SceneComponent.RelativeScale3D` (`self.Core`))) false false))))

(event `self.ReceiveTick`
  (params (DeltaSeconds :type "Float (single-precision)"))
  (`self.Floating`)
  (`KismetSystemLibrary.Delay` (`KismetMathLibrary.RandomFloatInRange` 0.0 2.0)))

(event `Floating`
  (bind _boule (`self.Boule`))
  (bind _boule_2 (`self.Boule`))
  (bind _returnvalue (`SceneComponent.GetRelativeTransform` _boule))
  (bind _returnvalue_2 (`SceneComponent.GetRelativeTransform` _boule_2))
  (`KismetSystemLibrary.MoveComponentTo` _boule (`KismetMathLibrary.MakeVector` (.x (.location _returnvalue)) (.y (.location _returnvalue)) (+ (.z (.location _returnvalue)) 10.0)) (.rotation _returnvalue) true true 1.0)
  (`KismetSystemLibrary.MoveComponentTo` _boule_2 (`KismetMathLibrary.MakeVector` (.x (.location _returnvalue_2)) (.y (.location _returnvalue_2)) (+ (.z (.location _returnvalue_2)) -10.0)) (.rotation _returnvalue_2) true true 1.0))

(event `FloatingBoat`
  (bind _zodiac (`self.Zodiac`))
  (bind _zodiac_2 (`self.Zodiac`))
  (bind _returnvalue (`SceneComponent.GetRelativeTransform` _zodiac))
  (bind _returnvalue_2 (`SceneComponent.GetRelativeTransform` _zodiac_2))
  (`KismetSystemLibrary.MoveComponentTo` _zodiac (`KismetMathLibrary.MakeVector` (.x (.location _returnvalue)) (.y (.location _returnvalue)) (+ (.z (.location _returnvalue)) 10.0)) (.rotation _returnvalue) true true 1.0)
  (`KismetSystemLibrary.MoveComponentTo` _zodiac_2 (`KismetMathLibrary.MakeVector` (.x (.location _returnvalue_2)) (.y (.location _returnvalue_2)) (+ (.z (.location _returnvalue_2)) -10.0)) (.rotation _returnvalue_2) true true 1.0))

(fn `UserConstructionScript`)