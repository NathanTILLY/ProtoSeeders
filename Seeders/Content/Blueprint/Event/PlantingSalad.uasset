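; Event actor that plays a timed lettuce-planting sequence by swapping which lettuce component is visible.
; On BeginPlay two delays run in parallel: after about 1.6 seconds the table lettuce hides and the hand ("Main") lettuce appears.
; At about 3.9 seconds the hand lettuce component is destroyed and the ground ("Sol") lettuce is shown.
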(event `self.ReceiveBeginPlay`
  (`|ExecutionSequence`
    (:`then_0`
      (`KismetSystemLibrary.Delay` 1.58749)
      (`|ExecutionSequence`
        (:`then_0`
          (`SceneComponent.SetVisibility` (`self.LettuceTable`) false false))
        (:`then_1`
          (`SceneComponent.SetVisibility` (`self.SM_KB3D_DMZ_Lettuce_B_Main`) true false))))
    (:`then_1`
      (`KismetSystemLibrary.Delay` 3.932634)
      (`|ExecutionSequence`
        (:`then_0`
          (`ActorComponent.K2_DestroyComponent` (`self.SM_KB3D_DMZ_Lettuce_B_Main`)))
        (:`then_1`
          (`SceneComponent.SetVisibility` (`self.LettuceSol`) true false))))))

(fn `UserConstructionScript`)