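; BP_JohnnyNPC is an NPC character Blueprint that randomizes its appearance and walk speed for visual and movement variety.
; Its construction script independently rolls one of three materials each for the jacket, pants and beanie, applying them to separate mesh slots.
; It also sets a random max walk speed on the movement component.
; Randomization re-rolls whenever the construction script runs, and the event graph holds no active logic.
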(fn `UserConstructionScript`
  (`|ExecutionSequence`
    (:`then_0`
      ;[1 1 1] Veste
      (set `self.RandIntTop` (`KismetMathLibrary.RandomIntegerInRange` 0 2))
      (`|ExecutionSequence`
        (:`then_0`
          (if (== (`self.RandIntTop`) 0)
            (`PrimitiveComponent.SetMaterial` (`self.Mesh`) 1 "/Game/Animations/Hobo/Materials/Top1.Top1")))
        (:`then_1`
          (if (== (`self.RandIntTop`) 1)
            (`PrimitiveComponent.SetMaterial` (`self.Mesh`) 1 "/Game/Animations/Hobo/Materials/Top2.Top2")))
        (:`then_2`
          (if (== (`self.RandIntTop`) 2)
            (`PrimitiveComponent.SetMaterial` (`self.Mesh`) 1 "/Game/Animations/Hobo/Materials/Top3.Top3")))))
    (:`then_1`
      ;[1 1 1] Pantalmon
      (set `self.RandIntBottom` (`KismetMathLibrary.RandomIntegerInRange` 0 2))
      (`|ExecutionSequence`
        (:`then_0`
          (if (== (`self.RandIntBottom`) 0)
            (`PrimitiveComponent.SetMaterial` (`self.Mesh`) 7 "/Game/Animations/Hobo/Materials/Bottom1.Bottom1")))
        (:`then_1`
          (if (== (`self.RandIntBottom`) 1)
            (`PrimitiveComponent.SetMaterial` (`self.Mesh`) 7 "/Game/Animations/Hobo/Materials/Bottom2.Bottom2")))
        (:`then_2`
          (if (== (`self.RandIntBottom`) 2)
            (`PrimitiveComponent.SetMaterial` (`self.Mesh`) 7 "/Game/Animations/Hobo/Materials/Bottom3.Bottom3")))))
    (:`then_2`
      ;[1 1 1] Bonnet
      (set `self.RandIntHat` (`KismetMathLibrary.RandomIntegerInRange` 0 2))
      (`|ExecutionSequence`
        (:`then_0`
          (if (== (`self.RandIntHat`) 0)
            (`PrimitiveComponent.SetMaterial` (`self.Mesh`) 2 "/Game/Animations/Hobo/Materials/Hat1.Hat1")))
        (:`then_1`
          (if (== (`self.RandIntHat`) 1)
            (`PrimitiveComponent.SetMaterial` (`self.Mesh`) 2 "/Game/Animations/Hobo/Materials/Hat2.Hat2")))
        (:`then_2`
          (if (== (`self.RandIntHat`) 2)
            (`PrimitiveComponent.SetMaterial` (`self.Mesh`) 2 "/Game/Animations/Hobo/Materials/Hat3.Hat3")))))
    (:`then_3`
      (set `CharacterMovementComponent.MaxWalkSpeed` (`KismetMathLibrary.RandomFloatInRange` 170.0 270.0) (`self.CharacterMovement`)))))