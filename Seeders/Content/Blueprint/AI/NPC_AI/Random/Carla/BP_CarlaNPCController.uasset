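; AI controller for the Carla NPC that runs its behavior tree, BT_CarlaNPC, after an optional start delay taken from the pawn.
; Shortly after starting, it copies the pawn's random-or-controlled flag into the blackboard.
; GoThroughCheckpoints writes the next checkpoint location from the pawn's list to the DefinedLocation key and advances an index, stopping at the list's end.
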(event `self.ReceiveBeginPlay`
  (bind _asbp_carla_npc (cast `/Game/Blueprint/AI/NPC_AI/Random/Carla/BP_CarlaNPC` (`self.K2_GetPawn`) :!pure true))
  (`KismetSystemLibrary.Delay` 0.1)
  (if (`/Game/Blueprint/AI/NPC_AI/BP_ParentNPC.WaitTime` _asbp_carla_npc)
    (`KismetSystemLibrary.Delay` (`/Game/Blueprint/AI/NPC_AI/BP_ParentNPC.WaitDuration` _asbp_carla_npc)))
  ;[1 0.159 0] WhenCopyingChangeThat
  (`self.RunBehaviorTree` "/Game/Blueprint/AI/NPC_AI/Random/Carla/BT_CarlaNPC.BT_CarlaNPC")
  ;[1 1 1] Handle wheter random or controlled
  (`KismetSystemLibrary.Delay` 0.2)
  (`BlackboardComponent.SetValueAsBool` (`AIBlueprintHelperLibrary.GetBlackboard` null) "RandomTrueOrControlledFalse" (`/Game/Blueprint/AI/NPC_AI/BP_ParentNPC.RandomTrueOrControlledFalse` (cast `/Game/Blueprint/AI/NPC_AI/Random/Carla/BP_CarlaNPC` (`self.K2_GetPawn`) :!pure true))))

(event `GoThroughCheckpoints`
  (bind _checkpoints (`/Game/Blueprint/AI/NPC_AI/BP_ParentNPC.Checkpoints` (cast `/Game/Blueprint/AI/NPC_AI/Random/Carla/BP_CarlaNPC` (`self.K2_GetPawn`) :!pure true)))
  (if (not (>= (`self.incrementationList`) (`KismetArrayLibrary.Array_Length` _checkpoints)))
    (`BlackboardComponent.SetValueAsVector` (`AIBlueprintHelperLibrary.GetBlackboard` null) "DefinedLocation" (`self.K2_GetActorLocation` (`|GetArrayItem` _checkpoints (`self.incrementationList`))))
    (`/Engine/EditorBlueprintResources/StandardMacros.IncrementInt` (`self.incrementationList`))))

(fn `UserConstructionScript`
  (`parent.UserConstructionScript`))