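; Yakuza NPC Blueprint that randomizes its look and walking speed for variety.
; The Construction Script picks one of two outfits at random, black or pink, setting matching suit and shoe materials on the mesh.
; It also sets the CharacterMovement max walk speed to a random value between MinSpeed and MaxSpeed.
; The Event Graph holds only disabled default events, so this Blueprint adds no runtime logic there.
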(fn `UserConstructionScript`
  (`|ExecutionSequence`
    (:`then_0`
      (set `self.RandInt` (`KismetMathLibrary.RandomIntegerInRange` 0 1))
      (`|ExecutionSequence`
        (:`then_0`
          (if (== (`self.RandInt`) 0)
            (`PrimitiveComponent.SetMaterial` (`self.Mesh`) 9 "/Game/Animations/Yakuza/Materials/CostardNoir.CostardNoir")
            (`PrimitiveComponent.SetMaterial` (`self.Mesh`) 8 "/Game/Animations/Yakuza/Materials/ShoeNoir.ShoeNoir")))
        (:`then_1`
          (if (== (`self.RandInt`) 1)
            (`PrimitiveComponent.SetMaterial` (`self.Mesh`) 9 "/Game/Animations/Yakuza/Materials/CostardRose.CostardRose")
            (`PrimitiveComponent.SetMaterial` (`self.Mesh`) 8 "/Game/Animations/Yakuza/Materials/M_ShoeRose.M_ShoeRose")))))
    (:`then_1`
      (set `CharacterMovementComponent.MaxWalkSpeed` (`KismetMathLibrary.RandomFloatInRange` (`self.MinSpeed`) (`self.MaxSpeed`)) (`self.CharacterMovement`)))))