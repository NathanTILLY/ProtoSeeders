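; AI controller for BP_AfricanOtherManNPC that drives its random or checkpoint-controlled behavior.
; On BeginPlay it optionally waits for the pawn's configured duration, runs BT_AfricanOtherManNPC, then copies the random/controlled flag to the blackboard.
; Each GoThroughCheckpoints call writes the next checkpoint location to DefinedLocation, setting Clapping? once the list is exhausted.
; Comments flag the NPC-specific references to change when copying the controller.
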(event `self.ReceiveBeginPlay`
  (bind _asbp_african_other_man_npc (cast `/Game/Blueprint/AI/NPC_AI/Random/AfricanMan/OtherMan/BP_AfricanOtherManNPC` (`self.K2_GetPawn`) :!pure true))
  (`KismetSystemLibrary.Delay` 0.1)
  (if (`/Game/Blueprint/AI/NPC_AI/BP_ParentNPC.WaitTime` _asbp_african_other_man_npc)
    (`KismetSystemLibrary.Delay` (`/Game/Blueprint/AI/NPC_AI/BP_ParentNPC.WaitDuration` _asbp_african_other_man_npc)))
  ;[1 0.159 0] WhenCopyingChangeThat
  (`self.RunBehaviorTree` "/Game/Blueprint/AI/NPC_AI/Random/AfricanMan/OtherMan/BT_AfricanOtherManNPC.BT_AfricanOtherManNPC")
  ;[1 1 1] Handle wheter random or controlled
  (`KismetSystemLibrary.Delay` 0.2)
  (`BlackboardComponent.SetValueAsBool` (`AIBlueprintHelperLibrary.GetBlackboard` null) "RandomTrueOrControlledFalse" (`/Game/Blueprint/AI/NPC_AI/BP_ParentNPC.RandomTrueOrControlledFalse` (cast `/Game/Blueprint/AI/NPC_AI/Random/AfricanMan/OtherMan/BP_AfricanOtherManNPC` (`self.K2_GetPawn`) :!pure true))))

(event `GoThroughCheckpoints`
  (bind _returnvalue (`AIBlueprintHelperLibrary.GetBlackboard` null))
  (bind _checkpoints (`/Game/Blueprint/AI/NPC_AI/BP_ParentNPC.Checkpoints` (cast `/Game/Blueprint/AI/NPC_AI/Random/AfricanMan/OtherMan/BP_AfricanOtherManNPC` (`self.K2_GetPawn`) :!pure true)))
  (if (>= (`self.incrementationList`) (`KismetArrayLibrary.Array_Length` _checkpoints))
    (`BlackboardComponent.SetValueAsBool` _returnvalue "Clapping?" true)
    (else
      (`BlackboardComponent.SetValueAsVector` _returnvalue "DefinedLocation" (`self.K2_GetActorLocation` (`|GetArrayItem` _checkpoints (`self.incrementationList`))))
      (`/Engine/EditorBlueprintResources/StandardMacros.IncrementInt` (`self.incrementationList`)))))

(fn `UserConstructionScript`
  (`parent.UserConstructionScript`))