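; BP_BrasilianNPC is a Brazilian-themed AI NPC character that varies its appearance and walking speed per instance.
; The construction script randomly picks one of three materials for a single mesh slot and sets a random max walk speed.
; Its event graph holds only disabled default events, so it adds no runtime logic of its own.
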(fn `UserConstructionScript`
  (`|ExecutionSequence`
    (:`then_0`
      (set `self.RandInt` (`KismetMathLibrary.RandomIntegerInRange` 0 2))
      (`|ExecutionSequence`
        (:`then_0`
          (if (== (`self.RandInt`) 0)
            (`PrimitiveComponent.SetMaterial` (`self.Mesh`) 4 "/Game/Animations/Brasilian/Materials/avaturn_look_0_material.avaturn_look_0_material")))
        (:`then_1`
          (if (== (`self.RandInt`) 1)
            (`PrimitiveComponent.SetMaterial` (`self.Mesh`) 4 "/Game/Animations/Brasilian/Materials/BrasilianBluieBlack.BrasilianBluieBlack")))
        (:`then_2`
          (if (== (`self.RandInt`) 2)
            (`PrimitiveComponent.SetMaterial` (`self.Mesh`) 4 "/Game/Animations/Brasilian/Materials/BrasilianGreenGrey.BrasilianGreenGrey")))))
    (:`then_1`
      (set `CharacterMovementComponent.MaxWalkSpeed` (`KismetMathLibrary.RandomFloatInRange` 170.0 270.0) (`self.CharacterMovement`)))))