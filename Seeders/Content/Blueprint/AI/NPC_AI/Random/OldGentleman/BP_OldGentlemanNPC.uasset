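; Old gentleman NPC Blueprint that adds a companion BP_AiActor when play begins.
; After the parent BeginPlay, it spawns that actor at a small offset from its capsule, matching the capsule's rotation.
; It then calls AttachActorToActor on the spawned actor with relative rules, but no parent actor is specified.
; Overlap, Tick and construction add no logic of their own.
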(event `self.ReceiveBeginPlay`
  (bind _capsulecomponent (`self.CapsuleComponent`))
  (`parent.ReceiveBeginPlay`)
  (bind _returnvalue (`|SpawnActorFromClass` "/Game/Blueprint/AI/PlayerAI/BP_AiActor.BP_AiActor_C" (`KismetMathLibrary.MakeTransform` (+ (`SceneComponent.K2_GetComponentLocation` _capsulecomponent) (50.0 50.0 50.0)) (`SceneComponent.K2_GetComponentRotation` _capsulecomponent)) "Undefined" "MultiplyWithRoot" null null))
  (`self.K2_AttachToActor` _returnvalue null "None" "KeepRelative" "KeepRelative" "KeepRelative" true))

(fn `UserConstructionScript`
  (`parent.UserConstructionScript`))