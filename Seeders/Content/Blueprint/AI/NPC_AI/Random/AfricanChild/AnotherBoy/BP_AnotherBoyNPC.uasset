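; BP_AnotherBoyNPC is an NPC character Blueprint in the random AfricanChild AI set.
; Its construction script sets the Character Movement max walk speed to a random value between MinSpeed and MaxSpeed, varying walk speed between instances.
; The event graph holds only disabled default events, so it adds no runtime logic of its own.
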(fn `UserConstructionScript`
  (set `CharacterMovementComponent.MaxWalkSpeed` (`KismetMathLibrary.RandomFloatInRange` (`self.MinSpeed`) (`self.MaxSpeed`)) (`self.CharacterMovement`)))