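; Adam NPC Blueprint that gives the character a randomized look.
; The Construction Script rolls a random integer and applies one of three Ch08 material variants to the second material slot of the mesh.
; The roll is unseeded, so the look can change whenever construction reruns.
; The Event Graph holds only disabled placeholder events, so this Blueprint adds no runtime logic of its own.
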(fn `UserConstructionScript`
  (set `self.RandInt` (`KismetMathLibrary.RandomIntegerInRange` 0 2))
  (`|ExecutionSequence`
    (:`then_0`
      (if (== (`self.RandInt`) 0)
        (`PrimitiveComponent.SetMaterial` (`self.Mesh`) 1 "/Game/Animations/AdamSurvetBlanc/Material/M_Ch08_OtherSurvetBleu.M_Ch08_OtherSurvetBleu")))
    (:`then_1`
      (if (== (`self.RandInt`) 1)
        (`PrimitiveComponent.SetMaterial` (`self.Mesh`) 1 "/Game/Animations/AdamSurvetBlanc/Material/M_Ch08_body1.M_Ch08_body1")))
    (:`then_2`
      (if (== (`self.RandInt`) 2)
        (`PrimitiveComponent.SetMaterial` (`self.Mesh`) 1 "/Game/Animations/AdamSurvetBlanc/Material/M_Ch08_OtherSurvet.M_Ch08_OtherSurvet")))))