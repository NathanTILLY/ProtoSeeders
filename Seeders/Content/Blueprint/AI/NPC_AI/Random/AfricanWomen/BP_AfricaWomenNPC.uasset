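; BP_AfricaWomenNPC is an NPC character Blueprint that gives each instance a randomized appearance and walk speed.
; Its construction script rolls one of three looks and swaps the outfit and shoe materials on two mesh slots to match.
; The same script sets the movement component's max walk speed to a random value between MinSpeed and MaxSpeed.
; The event graph holds only disabled default events.
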(fn `UserConstructionScript`
  (set `self.RandInt` (`KismetMathLibrary.RandomIntegerInRange` 0 2))
  (`|ExecutionSequence`
    (:`then_0`
      (if (== (`self.RandInt`) 0)
        (`PrimitiveComponent.SetMaterial` (`self.Mesh`) 9 "/Game/Animations/BrasilianWoman/Materials/avaturn_look_0_material.avaturn_look_0_material")
        (`PrimitiveComponent.SetMaterial` (`self.Mesh`) 8 "/Game/Animations/BrasilianWoman/Materials/avaturn_shoes_0_material.avaturn_shoes_0_material")))
    (:`then_1`
      (if (== (`self.RandInt`) 1)
        (`PrimitiveComponent.SetMaterial` (`self.Mesh`) 9 "/Game/Animations/BrasilianWoman/Materials/JacketAndPants.JacketAndPants")
        (`PrimitiveComponent.SetMaterial` (`self.Mesh`) 8 "/Game/Animations/BrasilianWoman/Materials/avaturn_shoes_0_material.avaturn_shoes_0_material")))
    (:`then_2`
      (if (== (`self.RandInt`) 2)
        (`PrimitiveComponent.SetMaterial` (`self.Mesh`) 9 "/Game/Animations/BrasilianWoman/Materials/JacketAndPantsBlue.JacketAndPantsBlue")
        (`PrimitiveComponent.SetMaterial` (`self.Mesh`) 8 "/Game/Animations/BrasilianWoman/Materials/ShoesBlack.ShoesBlack")))
    (:`then_3`
      (set `CharacterMovementComponent.MaxWalkSpeed` (`KismetMathLibrary.RandomFloatInRange` (`self.MinSpeed`) (`self.MaxSpeed`)) (`self.CharacterMovement`)))))