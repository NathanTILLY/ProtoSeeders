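; AI controller for the MathisGang NPC that starts its behavior tree and supplies patrol checkpoints.
; BeginPlay runs BT_MathisGangNPC after a brief delay, plus an optional wait configured on the pawn.
; GoThroughCheckpoints writes the pawn's next checkpoint location to the DefinedLocation blackboard key, advancing without looping.
; The random-versus-controlled blackboard write is unconnected; comments flag NPC-specific nodes to change when copying.
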(event `self.ReceiveBeginPlay`
  (bind _asbp_mathis_gang_npc (cast `/Game/Blueprint/AI/NPC_AI/Us/MathisGang/BP_MathisGangNPC` (`self.K2_GetPawn`) :!pure true))
  (`KismetSystemLibrary.Delay` 0.1)
  (if (`/Game/Blueprint/AI/NPC_AI/BP_ParentNPC.WaitTime` _asbp_mathis_gang_npc)
    (`KismetSystemLibrary.Delay` (`/Game/Blueprint/AI/NPC_AI/BP_ParentNPC.WaitDuration` _asbp_mathis_gang_npc)))
  ;[1 0.159 0] WhenCopyingChangeThat
  (`self.RunBehaviorTree` "/Game/Blueprint/AI/NPC_AI/Us/MathisGang/BT_MathisGangNPC.BT_MathisGangNPC"))

(event `GoThroughCheckpoints`
  (bind _checkpoints (`/Game/Blueprint/AI/NPC_AI/BP_ParentNPC.Checkpoints` (cast `/Game/Blueprint/AI/NPC_AI/Us/MathisGang/BP_MathisGangNPC` (`self.K2_GetPawn`) :!pure true)))
  (if (not (>= (`self.incrementationList`) (`KismetArrayLibrary.Array_Length` _checkpoints)))
    (`BlackboardComponent.SetValueAsVector` (`AIBlueprintHelperLibrary.GetBlackboard` null) "DefinedLocation" (`self.K2_GetActorLocation` (`|GetArrayItem` _checkpoints (`self.incrementationList`))))
    (`/Engine/EditorBlueprintResources/StandardMacros.IncrementInt` (`self.incrementationList`))))

(fn `UserConstructionScript`
  (`parent.UserConstructionScript`))