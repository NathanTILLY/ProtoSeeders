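; BP_MathisGangNPC is a Mathis gang NPC Blueprint that randomizes its look for visual variety.
; The Construction Script swaps materials on fixed mesh slots, picking one of three shirts and separately rolling for bald or haired.
; Two of the three hair rolls share the same material, so bald is the rarer result.
; The unseeded rolls can change whenever construction reruns, and the Event Graph holds no active logic.
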(fn `UserConstructionScript`
  (`|ExecutionSequence`
    (:`then_0`
      (set `self.RandInt` (`KismetMathLibrary.RandomIntegerInRange` 0 2))
      (`|ExecutionSequence`
        (:`then_0`
          (if (== (`self.RandInt`) 0)
            (`PrimitiveComponent.SetMaterial` (`self.Mesh`) 9 "/Game/Animations/MathisGang/Materials/M_MathisBaseShirt.M_MathisBaseShirt")))
        (:`then_1`
          (if (== (`self.RandInt`) 1)
            (`PrimitiveComponent.SetMaterial` (`self.Mesh`) 9 "/Game/Animations/MathisGang/Materials/M_MathisL2BShirt.M_MathisL2BShirt")))
        (:`then_2`
          (if (== (`self.RandInt`) 2)
            (`PrimitiveComponent.SetMaterial` (`self.Mesh`) 9 "/Game/Animations/MathisGang/Materials/M_MathisRGangShirt1.M_MathisRGangShirt1")))))
    (:`then_1`
      (set `self.RandIntHair` (`KismetMathLibrary.RandomIntegerInRange` 0 2))
      (`|ExecutionSequence`
        (:`then_0`
          (if (== (`self.RandIntHair`) 0)
            (`PrimitiveComponent.SetMaterial` (`self.Mesh`) 7 "/Game/Animations/MathisGang/Materials/M_HairBald.M_HairBald")
            (`PrimitiveComponent.SetMaterial` (`self.Mesh`) 6 "/Game/Animations/MathisGang/Materials/M_HairBald.M_HairBald")))
        (:`then_1`
          (if (== (`self.RandIntHair`) 1)
            (`PrimitiveComponent.SetMaterial` (`self.Mesh`) 7 "/Game/Animations/MathisGang/Materials/avaturn_hair_1_material.avaturn_hair_1_material")
            (`PrimitiveComponent.SetMaterial` (`self.Mesh`) 6 "/Game/Animations/MathisGang/Materials/avaturn_hair_1_material.avaturn_hair_1_material")))
        (:`then_2`
          (if (== (`self.RandIntHair`) 2)
            (`PrimitiveComponent.SetMaterial` (`self.Mesh`) 7 "/Game/Animations/Nathan/avaturn_hair_1_material.avaturn_hair_1_material")
            (`PrimitiveComponent.SetMaterial` (`self.Mesh`) 6 "/Game/Animations/Nathan/avaturn_hair_1_material.avaturn_hair_1_material")))))))