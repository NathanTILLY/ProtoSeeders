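; AI controller for the PetitTomSquidGame NPC that starts its behavior tree and feeds it movement data.
; On BeginPlay it optionally waits for the pawn's configured delay, runs BT_PetitTomSquidGameNpc, then copies the pawn's random-or-controlled flag to the blackboard.
; GoThroughCheckpoints writes the next checkpoint's location to DefinedLocation and advances an index until the list runs out.
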(event `self.ReceiveBeginPlay`
  (bind _aspetit_tom_squid_game (cast `/Game/Blueprint/AI/NPC_AI/Us/PetitTomSquidGame/PetitTomSquidGame` (`self.K2_GetPawn`) :!pure true))
  (`KismetSystemLibrary.Delay` 0.1)
  (if (`/Game/Blueprint/AI/NPC_AI/BP_ParentNPC.WaitTime` _aspetit_tom_squid_game)
    (`KismetSystemLibrary.Delay` (`/Game/Blueprint/AI/NPC_AI/BP_ParentNPC.WaitDuration` _aspetit_tom_squid_game)))
  ;[1 0.159 0] WhenCopyingChangeThat
  (`self.RunBehaviorTree` "/Game/Blueprint/AI/NPC_AI/Us/PetitTomSquidGame/BT_PetitTomSquidGameNpc.BT_PetitTomSquidGameNpc")
  ;[1 1 1] Handle wheter random or controlled
  (`KismetSystemLibrary.Delay` 0.2)
  (`BlackboardComponent.SetValueAsBool` (`AIBlueprintHelperLibrary.GetBlackboard` null) "RandomTrueOrControlledFalse" (`/Game/Blueprint/AI/NPC_AI/BP_ParentNPC.RandomTrueOrControlledFalse` (cast `/Game/Blueprint/AI/NPC_AI/Us/PetitTomSquidGame/PetitTomSquidGame` (`self.K2_GetPawn`) :!pure true))))

(event `GoThroughCheckpoints`
  (bind _checkpoints (`/Game/Blueprint/AI/NPC_AI/BP_ParentNPC.Checkpoints` (cast `/Game/Blueprint/AI/NPC_AI/Us/PetitTomSquidGame/PetitTomSquidGame` (`self.K2_GetPawn`) :!pure true)))
  (if (not (>= (`self.incrementationList`) (`KismetArrayLibrary.Array_Length` _checkpoints)))
    (`BlackboardComponent.SetValueAsVector` (`AIBlueprintHelperLibrary.GetBlackboard` null) "DefinedLocation" (`self.K2_GetActorLocation` (`|GetArrayItem` _checkpoints (`self.incrementationList`))))
    (`/Engine/EditorBlueprintResources/StandardMacros.IncrementInt` (`self.incrementationList`))))

(fn `UserConstructionScript`
  (`parent.UserConstructionScript`))