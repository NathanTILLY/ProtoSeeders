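; BP_NathanOGNPCController is the AI controller for the NathanOG NPC, switching it between random and controlled behavior.
; On BeginPlay it runs BT_NathanOGNPC, then after a short delay copies the pawn's random-or-controlled flag to the Blackboard.
; GoThroughCheckpoints writes the next checkpoint actor's location to DefinedLocation and advances the index, without looping after the last.
; "WhenCopyingChangeThat" notes mark the NPC-specific references to change when duplicating the controller.
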(event `self.ReceiveBeginPlay`
  ;[1 0.159 0] WhenCopyingChangeThat
  (`self.RunBehaviorTree` "/Game/Blueprint/AI/NPC_AI/Us/NathanOG/BT_NathanOGNPC.BT_NathanOGNPC")
  ;[1 1 1] Handle wheter random or controlled
  (`KismetSystemLibrary.Delay` 0.2)
  (`BlackboardComponent.SetValueAsBool` (`AIBlueprintHelperLibrary.GetBlackboard` null) "RandomTrueOrControlledFalse" (`/Game/Blueprint/AI/NPC_AI/BP_ParentNPC.RandomTrueOrControlledFalse` (cast `/Game/Blueprint/AI/NPC_AI/Us/NathanOG/BP_NathanOGNPC` (`self.K2_GetPawn`) :!pure true))))

(event `GoThroughCheckpoints`
  (bind _checkpoints (`/Game/Blueprint/AI/NPC_AI/BP_ParentNPC.Checkpoints` (cast `/Game/Blueprint/AI/NPC_AI/Us/NathanOG/BP_NathanOGNPC` (`self.K2_GetPawn`) :!pure true)))
  (if (not (>= (`self.incrementationList`) (`KismetArrayLibrary.Array_Length` _checkpoints)))
    (`BlackboardComponent.SetValueAsVector` (`AIBlueprintHelperLibrary.GetBlackboard` null) "DefinedLocation" (`self.K2_GetActorLocation` (`|GetArrayItem` _checkpoints (`self.incrementationList`))))
    (`/Engine/EditorBlueprintResources/StandardMacros.IncrementInt` (`self.incrementationList`))))

(fn `UserConstructionScript`
  (`parent.UserConstructionScript`))