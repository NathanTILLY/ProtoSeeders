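; BP_TomNPCController is the AI controller for the Tom NPC, starting the BT_NPCTom behavior tree on BeginPlay.
; Its GoToSphereLocation event casts the controlled pawn to BP_TomNPC and copies the location of that pawn's LocationToGo actor into the DefinedLocation blackboard key.
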(event `self.ReceiveBeginPlay`
  (`self.RunBehaviorTree` "/Game/Blueprint/AI/NPC_AI/Us/Tom/BT_NPCTom.BT_NPCTom"))

(event `GoToSphereLocation`
  (bind (_returnvalue_x _returnvalue_y _returnvalue_z) (`KismetMathLibrary.BreakVector` (`self.K2_GetActorLocation` (`/Game/Blueprint/AI/NPC_AI/Us/Tom/BP_TomNPC.LocationToGo` (cast `/Game/Blueprint/AI/NPC_AI/Us/Tom/BP_TomNPC` (`self.K2_GetPawn`) :!pure true)))))
  (`BlackboardComponent.SetValueAsVector` (`AIBlueprintHelperLibrary.GetBlackboard` null) "DefinedLocation" (`KismetMathLibrary.MakeVector` _returnvalue_x _returnvalue_y _returnvalue_z)))

(fn `UserConstructionScript`
  (`parent.UserConstructionScript`))