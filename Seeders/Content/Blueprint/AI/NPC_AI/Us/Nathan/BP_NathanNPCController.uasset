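; AI controller for the Nathan NPC that runs its behavior tree and feeds it patrol checkpoints for an inspection route.
; BeginPlay starts BT_NPCNathan.
; Each GoThroughCheckpoints call writes the next location from the pawn's Checkpoints array to the DefinedLocation blackboard key and advances the index.
; Once the index reaches the last element, it sets InspectionDone instead, so that final checkpoint is never written.
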(event `self.ReceiveBeginPlay`
  (`self.RunBehaviorTree` "/Game/Blueprint/AI/NPC_AI/Us/Nathan/BT_NPCNathan.BT_NPCNathan"))

(event `GoThroughCheckpoints`
  (bind _checkpoints (`/Game/Blueprint/AI/NPC_AI/BP_ParentNPC.Checkpoints` (cast `/Game/Blueprint/AI/NPC_AI/Us/Nathan/BP_NathanNPC` (`self.K2_GetPawn`) :!pure true)))
  (if (>= (`self.incrementationList`) (- (`KismetArrayLibrary.Array_Length` _checkpoints) 1))
    (`BlackboardComponent.SetValueAsBool` (`AIBlueprintHelperLibrary.GetBlackboard` null) "InspectionDone" true)
    (else
      (`BlackboardComponent.SetValueAsVector` (`AIBlueprintHelperLibrary.GetBlackboard` null) "DefinedLocation" (`self.K2_GetActorLocation` (`|GetArrayItem` _checkpoints (`self.incrementationList`))))
      (`/Engine/EditorBlueprintResources/StandardMacros.IncrementInt` (`self.incrementationList`)))))

(fn `UserConstructionScript`
  (`parent.UserConstructionScript`))