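; Character Blueprint for the Tom CPR NPC, which exposes a custom event for a timed CPR action.
; DoCPRevent raises the DoCPR flag, holds it through a fixed delay of roughly nine seconds, then clears it and sets a new max walk speed.
; A direct mesh animation call for a run-to-CPR asset is left unconnected, and BeginPlay, overlap and construction add no logic of their own.
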(event `DoCPRevent`
  (set `self.DoCPR` true)
  (`KismetSystemLibrary.Delay` 8.63)
  (set `self.DoCPR` false)
  (set `CharacterMovementComponent.MaxWalkSpeed` 1000.0 (`self.CharacterMovement`)))

(fn `UserConstructionScript`
  (`parent.UserConstructionScript`))