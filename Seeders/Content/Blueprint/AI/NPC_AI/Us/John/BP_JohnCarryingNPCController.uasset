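; AI controller for the John carrying NPC, which moves either randomly or along designer-set checkpoints.
; On BeginPlay it waits briefly, plus an optional pawn-defined delay, then runs BT_JohnCarryingNPC and copies the pawn's random-or-controlled flag to the Blackboard.
; GoThroughCheckpoints writes the next checkpoint's location to DefinedLocation and advances the index, stopping after the last.
; Pawn-specific casts and tree references are marked to change when copying.
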(event `self.ReceiveBeginPlay`
  (bind _asbp_john_npccarrying (cast `/Game/Blueprint/AI/NPC_AI/Us/John/BP_JohnNPCCarrying` (`self.K2_GetPawn`) :!pure true))
  (`KismetSystemLibrary.Delay` 0.1)
  (if (`/Game/Blueprint/AI/NPC_AI/BP_ParentNPC.WaitTime` _asbp_john_npccarrying)
    (`KismetSystemLibrary.Delay` (`/Game/Blueprint/AI/NPC_AI/BP_ParentNPC.WaitDuration` _asbp_john_npccarrying)))
  ;[1 0.159 0] WhenCopyingChangeThat
  (`self.RunBehaviorTree` "/Game/Blueprint/AI/NPC_AI/Us/John/BT_JohnCarryingNPC.BT_JohnCarryingNPC")
  ;[1 1 1] Handle wheter random or controlled
  (`BlackboardComponent.SetValueAsBool` (`AIBlueprintHelperLibrary.GetBlackboard` null) "RandomTrueOrControlledFalse" (`/Game/Blueprint/AI/NPC_AI/BP_ParentNPC.RandomTrueOrControlledFalse` (cast `/Game/Blueprint/AI/NPC_AI/Us/John/BP_JohnNPCCarrying` (`self.K2_GetPawn`) :!pure true))))

(event `GoThroughCheckpoints`
  (bind _checkpoints (`/Game/Blueprint/AI/NPC_AI/BP_ParentNPC.Checkpoints` (cast `/Game/Blueprint/AI/NPC_AI/Us/John/BP_JohnNPCCarrying` (`self.K2_GetPawn`) :!pure true)))
  (if (not (>= (`self.incrementationList`) (`KismetArrayLibrary.Array_Length` _checkpoints)))
    (`BlackboardComponent.SetValueAsVector` (`AIBlueprintHelperLibrary.GetBlackboard` null) "DefinedLocation" (`self.K2_GetActorLocation` (`|GetArrayItem` _checkpoints (`self.incrementationList`))))
    (`/Engine/EditorBlueprintResources/StandardMacros.IncrementInt` (`self.incrementationList`))))

(fn `UserConstructionScript`)