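; BP_AINPC is a floating orb (Boule) companion that attaches to a referenced NPC's head socket.
; Shortly after BeginPlay it attaches and places the orb at an offset from the NPC.
; Custom event Floating eases the orb up and down, while AIHoverplayer plays and reverses a timeline paced by PathDivisionTime.
; The hover path looks unfinished: its update only prints debug text and resets the orb's relative transform, leaving the Lerp unused.
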(event `self.ReceiveBeginPlay`
  (`KismetSystemLibrary.Delay` 0.0002)
  (`self.K2_AttachToActor` (`self.NPCRef`) "HeadSocket" "KeepWorld" "KeepWorld" "KeepWorld")
  (`SceneComponent.K2_SetWorldLocation` (`self.Boule`) (+ (`self.K2_GetActorLocation` (`self.NPCRef`)) (0.0 75.0 75.0)) false false))

(event `Floating`
  (bind _boule (`self.Boule`))
  (bind _boule_2 (`self.Boule`))
  (bind _returnvalue (`SceneComponent.GetRelativeTransform` _boule_2))
  (bind _returnvalue_2 (`SceneComponent.GetRelativeTransform` _boule))
  (`KismetSystemLibrary.MoveComponentTo` _boule_2 (`KismetMathLibrary.MakeVector` (.x (.location _returnvalue)) (.y (.location _returnvalue)) (+ (.z (.location _returnvalue)) 10.0)) (.rotation _returnvalue) true true 1.0)
  (`KismetSystemLibrary.MoveComponentTo` _boule (`KismetMathLibrary.MakeVector` (.x (.location _returnvalue_2)) (.y (.location _returnvalue_2)) (+ (.z (.location _returnvalue_2)) -10.0)) (.rotation _returnvalue_2) true true 1.0))

(event `AIHoverplayer`
  (bind _boule (`self.Boule`))
  (`TimelineComponent.SetPlayRate` (`self.Timeline`) (/ 1.0 (`self.PathDivisionTime`)))
  (bind (_direction _alphaa) (`Timeline|Timeline` :!label _label)
    (:`Update`
      (`KismetSystemLibrary.PrintString` "Hello")
      (`SceneComponent.K2_SetRelativeTransform` _boule (`KismetMathLibrary.MakeTransform` (0.0 0.0 0.0) (`SceneComponent.RelativeRotation` _boule)) false false))
    (:`Finished`
      (`KismetSystemLibrary.Delay` 0.2)
      (goto _label :!via `Reverse`))))

(fn `UserConstructionScript`)