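; BP_AiActor is an actor that moves its Boule component along its own spline in a repeating loop.
; On BeginPlay it finds the BP_OldGentlemanNPC, attaches itself to it keeping its world transform, then starts OtherPath.
; OtherPath runs a Timeline whose alpha maps to distance along the spline in local space, setting Boule's relative location, and restarts after a short delay.
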(event `self.ReceiveBeginPlay`
  (`|ExecutionSequence`
    (:`then_0`
      (bind _returnvalue (`GameplayStatics.GetActorOfClass` "/Game/Blueprint/AI/NPC_AI/Random/OldGentleman/BP_OldGentlemanNPC.BP_OldGentlemanNPC_C"))
      (bind _output_get (set `self.NewVar` _returnvalue))
      (`self.K2_AttachToActor` _output_get "None" "KeepWorld" "KeepWorld" "KeepWorld"))
    (:`then_1`
      (`self.OtherPath`))))

(event `OtherPath`
  (bind (_direction _alphaa) (`Timeline|Timeline` :!label _label)
    (:`Update`
      (`SceneComponent.K2_SetRelativeLocation` (`self.Boule`) (`SplineComponent.GetLocationAtDistanceAlongSpline` (`self.Spline`) (`KismetMathLibrary.Lerp` 0.0 (`SplineComponent.GetSplineLength` (`self.Spline`)) _alphaa) "Local") false false))
    (:`Finished`
      (`KismetSystemLibrary.Delay` 0.2)
      (goto _label :!via `PlayFromStart`))))

(fn `UserConstructionScript`)